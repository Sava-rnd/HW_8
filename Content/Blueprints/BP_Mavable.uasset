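; BP_Mavable is a pawn that wanders endlessly between random points using AI movement, starting at BeginPlay.
; MoveTo applies Speed to the floating movement component and targets a random point in a box, using the Min values as center and Max as half-sizes.
; It repeats on success or failure, randomizing yaw after successes and printing the result.
; An older bounds-based variant is disconnected, and the 2D bounds helper is unused.
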(event `self.ReceiveBeginPlay`
  (`self.Move To`))

(event `Move To`
  (bind (_returnvalue_roll _returnvalue_pitch _returnvalue_yaw) (`KismetMathLibrary.BreakRotator` (`KismetMathLibrary.RandomRotator` false)))
  (`|ExecutionSequence`
    (:`then_0`
      (set `FloatingPawnMovement.MaxSpeed` (`self.Speed`) (`self.FloatingPawnMovement`))
      (set `self.TargetLocation` (`self.K2_GetActorLocation`))
      (bind _movementresult (`|AIMoveTo` self (`KismetMathLibrary.RandomPointInBoundingBox` (`KismetMathLibrary.MakeVector` (`self.Min X`) (`self.Min Y`)) (`KismetMathLibrary.MakeVector` (`self.Max X`) (`self.Max Y`))) null)
        (:`OnSuccess`
          (`self.K2_SetActorRotation` (`KismetMathLibrary.MakeRotator` 0.0 0.0 _returnvalue_yaw)))
        (:`OnFail`
          _))
      (`self.Move To`)
      (`KismetSystemLibrary.PrintString` (`|GetEnumeratorNameAsString` _movementresult)))))

(fn `Is Actor in Boundaries 2D`
  (params (`Min X` :type "Float (double-precision)") (`Max X` :type "Float (double-precision)") (`Min Y` :type "Float (double-precision)") (`Max Y` :type "Float (double-precision)"))
  (returns (ReturnValue :type Boolean))
  (bind (_returnvalue_x _returnvalue_y) (`KismetMathLibrary.BreakVector` (`self.K2_GetActorLocation`)))
  (return (and (`KismetMathLibrary.InRange_FloatFloat` _returnvalue_x `Min X` `Max X`) (`KismetMathLibrary.InRange_FloatFloat` _returnvalue_y `Min Y` `Max Y`))))

(fn `UserConstructionScript`)